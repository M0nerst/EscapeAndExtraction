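; Evacuation zone actor that runs a countdown while the player stands inside, once all shields are activated and key cards collected in GM_LeaveMeAlone.
; Overlap begin checks those requirements, then starts a looping timer that pushes elapsed time to the game mode's quest progress.
; Overlap end clears the timer and resets progress.
; Reaching the required time triggers the game mode's all-quests-completed check without stopping the timer.
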(event Custom|StartEvacuation
  (bind _asgm_leave_me_alone (Utilities|Casting|CastToGM_LeaveMeAlone (Game|GetGameMode)))
  (if (>= (Variables|/Game/LeaveMeAlone/Core/GameMode/GM_LeaveMeAlone.GM_LeaveMeAlone_C|GetShieldsActivated _asgm_leave_me_alone) (Variables|/Game/LeaveMeAlone/Core/GameMode/GM_LeaveMeAlone.GM_LeaveMeAlone_C|GetTotalShilds _asgm_leave_me_alone))
    (if (>= (Variables|/Game/LeaveMeAlone/Core/GameMode/GM_LeaveMeAlone.GM_LeaveMeAlone_C|GetKeyCardsCollected _asgm_leave_me_alone) (Variables|/Game/LeaveMeAlone/Core/GameMode/GM_LeaveMeAlone.GM_LeaveMeAlone_C|GetTotalKeyCards _asgm_leave_me_alone))
      (Variables|Default|SetCurrentTime 0.0)
      (bind _returnvalue (Utilities|Time|SetTimerbyFunctionName 0 "EvacuationTick" 0.1 true))
      (Variables|Default|SetEvacuationTimerHandle _returnvalue)
      (Development|PrintString "Эвакуация началась." true true "(R=0.000000,G=1.000000,B=0.097032,A=1.000000)" 1.0)
      (else
        (Development|PrintString "Собери все ключи.")))
    (else
      (Development|PrintString "Активируй все щиты."))))

(event Custom|StopEvacuation
  (Utilities|Time|ClearandInvalidateTimerbyHandle (Variables|Default|GetEvacuationTimerHandle))
  (Variables|Default|SetCurrentTime 0.0)
  (bind _asgm_leave_me_alone (Utilities|Casting|CastToGM_LeaveMeAlone (Game|GetGameMode)))
  (Variables|/Game/LeaveMeAlone/Core/GameMode/GM_LeaveMeAlone.GM_LeaveMeAlone_C|SetEvacuationTime _asgm_leave_me_alone 0.0)
  (Default|CallOnQuestProgressChanged _asgm_leave_me_alone))

(event Custom|EvacuationTick
  (if (and (not (Variables|Default|GetbIsPlayerInZone)) (Variables|Default|GetbIsEvacuated))
    (Utilities|Time|ClearandInvalidateTimerbyHandle (Variables|Default|GetEvacuationTimerHandle))
    (Variables|Default|SetCurrentTime 0.0)
    (else
      (Variables|Default|SetCurrentTime (+ (Variables|Default|GetCurrentTime) 0.1))
      (bind _asgm_leave_me_alone (Utilities|Casting|CastToGM_LeaveMeAlone (Game|GetGameMode)))
      (Variables|/Game/LeaveMeAlone/Core/GameMode/GM_LeaveMeAlone.GM_LeaveMeAlone_C|SetEvacuationTime _asgm_leave_me_alone (Variables|Default|GetCurrentTime))
      (Default|CallOnQuestProgressChanged _asgm_leave_me_alone)
      (if (>= (Variables|Default|GetCurrentTime) (Variables|Default|GetRequiredTime))
        (CallFunction|CompleteEvacuation)))))

(event Custom|CompleteEvacuation
  (bind _asgm_leave_me_alone (Utilities|Casting|CastToGM_LeaveMeAlone (Game|GetGameMode)))
  (Variables|/Game/LeaveMeAlone/Core/GameMode/GM_LeaveMeAlone.GM_LeaveMeAlone_C|SetEvacuationTime _asgm_leave_me_alone (Variables|Default|GetRequiredTime))
  (Default|CallOnQuestProgressChanged _asgm_leave_me_alone)
  (Default|CheckAllQuestsCompleted _asgm_leave_me_alone))

(event EventBeginPlay
  (bind _returnvalue (Class|LMAConfigLibrary|GetRequiredEvacuationTime))
  (Variables|Default|SetRequiredTime _returnvalue))

(event Collision|EventActorBeginOverlap
  (params (OtherActor :type Actor%20Object%20Reference))
  (if (Pawn|IsPlayerControlled (Variables|/Script/Engine.Actor|GetInstigator OtherActor))
    (Utilities|Casting|CastToLMADefaultCharacter (Game|GetPlayerCharacter 0))
    (Variables|Default|SetbIsPlayerInZone true)
    (CallFunction|StartEvacuation)))

(event EventTick
  (params (DeltaSeconds :type Float%20%28single-precision%29)))

(event Collision|EventActorEndOverlap
  (params (OtherActor :type Actor%20Object%20Reference))
  (if (Pawn|IsPlayerControlled (Variables|/Script/Engine.Actor|GetInstigator OtherActor))
    (Utilities|Casting|CastToLMADefaultCharacter (Game|GetPlayerCharacter 0))
    (if true
      (Variables|Default|SetbIsPlayerInZone false)
      (CallFunction|StopEvacuation))))

(fn ConstructionScript)