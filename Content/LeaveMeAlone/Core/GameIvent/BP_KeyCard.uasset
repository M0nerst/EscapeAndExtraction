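; BP_KeyCard is a collectible quest key card that cycles between active and hidden states.
; Looping back-and-forth timers toggle visibility and collision using TimeToLive and RespawnDelay from getters, with an extra TimeToAppear timer when starting inactive.
; A player-controlled overlap while active increments KeyCardsCollected on GM_LeaveMeAlone, triggers quest progress and completion checks, then destroys the actor.
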(event Custom|ActivateKey
  (Variables|Default|SetbIsActive true)
  (Rendering|SetVisibility (Variables|Default|GetDefaultSceneRoot) true true)
  (Collision|SetCollisionEnabled (Variables|Default|GetSphere) "QueryAndPhysics")
  (Collision|SetCollisionEnabled (Variables|Default|GetStaticMesh) "QueryAndPhysics")
  (Utilities|Time|SetTimerbyEvent (delegate Custom|DeactivateKey) (Variables|Default|GetTimeToLive)))

(event Custom|DeactivateKey
  (Variables|Default|SetbIsActive false)
  (Rendering|SetVisibility (Variables|Default|GetStaticMesh) false true)
  (Collision|SetCollisionEnabled (Variables|Default|GetSphere) "NoCollision")
  (Collision|SetCollisionEnabled (Variables|Default|GetStaticMesh) "NoCollision")
  (Utilities|Time|SetTimerbyEvent (delegate Custom|ActivateKey) (Variables|Default|GetRespawnDelay)))

(event EventBeginPlay
  (bind _returnvalue (Class|LMAConfigLibrary|GetKeyCardTTL))
  (Variables|Default|SetTimeToLive _returnvalue)
  (bind _returnvalue_2 (Class|LMAConfigLibrary|GetKeyCardRespawnDelay))
  (Variables|Default|SetRespawnDelay _returnvalue_2)
  (if (Variables|Default|GetbStartActive)
    (CallFunction|ActivateKey)
    (else
      (CallFunction|DeactivateKey)
      (Utilities|Time|SetTimerbyEvent (delegate Custom|ActivateKey) (Variables|Default|GetTimeToAppear)))))

(event Collision|EventActorBeginOverlap
  (params (OtherActor :type Actor%20Object%20Reference))
  (if (Pawn|IsPlayerControlled (Variables|/Script/Engine.Actor|GetInstigator OtherActor))
    (if (Variables|Default|GetbIsActive)
      (if (not (Variables|Default|GetbIsCollected))
        (Variables|Default|SetbIsCollected true)
        (bind _asgm_leave_me_alone (Utilities|Casting|CastToGM_LeaveMeAlone (Game|GetGameMode)))
        (Variables|/Game/LeaveMeAlone/Core/GameMode/GM_LeaveMeAlone.GM_LeaveMeAlone_C|SetKeyCardsCollected _asgm_leave_me_alone (+ (Variables|/Game/LeaveMeAlone/Core/GameMode/GM_LeaveMeAlone.GM_LeaveMeAlone_C|GetKeyCardsCollected _asgm_leave_me_alone) 1))
        (Default|CallOnQuestProgressChanged _asgm_leave_me_alone)
        (Default|CheckAllQuestsCompleted _asgm_leave_me_alone)
        (Actor|DestroyActor)))))

(event EventTick
  (params (DeltaSeconds :type Float%20%28single-precision%29)))

(fn ConstructionScript)