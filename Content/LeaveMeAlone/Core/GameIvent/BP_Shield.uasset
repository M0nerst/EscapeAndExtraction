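; BP_Shield is a quest objective actor, a shield that the player activates by overlapping it.
; On overlap, it checks that the other actor's instigator is player-controlled, then sets a one-time activation flag.
; First activation increments the shield count on GM_LeaveMeAlone, signals quest progress and requests an all-quests completion check.
; Later overlaps only print a Russian debug message saying the shield is already activated.
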(event Collision|EventActorBeginOverlap
  (params (OtherActor :type Actor%20Object%20Reference))
  (if (Pawn|IsPlayerControlled (Variables|/Script/Engine.Actor|GetInstigator OtherActor))
    (if (Variables|Default|GetbIsActivated)
      (Development|PrintString "Этот щит уже активирован." true true "(R=1.000000,G=0.012386,B=0.000000,A=1.000000)" 4.0)
      (else
        (Variables|Default|SetbIsActivated true)
        (bind _asgm_leave_me_alone (Utilities|Casting|CastToGM_LeaveMeAlone (Game|GetGameMode)))
        (Variables|/Game/LeaveMeAlone/Core/GameMode/GM_LeaveMeAlone.GM_LeaveMeAlone_C|SetShieldsActivated _asgm_leave_me_alone (+ (Variables|/Game/LeaveMeAlone/Core/GameMode/GM_LeaveMeAlone.GM_LeaveMeAlone_C|GetShieldsActivated _asgm_leave_me_alone) 1))
        (Default|CallOnQuestProgressChanged _asgm_leave_me_alone)
        (Default|CheckAllQuestsCompleted _asgm_leave_me_alone)))))

(fn ConstructionScript)